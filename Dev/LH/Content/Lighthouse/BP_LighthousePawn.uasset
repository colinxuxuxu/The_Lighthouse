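; Player pawn for the lighthouse, handling the searchlight, clickable key objects and the radio.
; Each tick it sphere-traces along the spotlight; ocean hits steer follower ships through AI blackboards and set any detected pirate chasing.
; Left-clicks open key-object popups and advance progression, while bound controller mouse events drive the radio slider, static noise and camera return.
; Debug keys are included; the son's ship capsize call is disconnected.
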(event Custom|ToggleSliderUI
  (Default|ToggleSlider (Variables|Default|GetRadioUI)))

(event Custom|ToggleSlider
  (bind _returnvalue (Subsystems|GetProgressionSubsystem))
  (bind _radiobackgroundnoise (Variables|Default|GetRadioBackgroundNoise))
  (bind _radioui (Variables|Default|GetRadioUI))
  (bind _currprogress (Variables|/Script/The_Lighthouse.ProgressionSubsystem|GetCurrProgress _returnvalue))
  (bind _isslideron (Variables|/Game/Ken_Playground/ClickableUI/WBP_Radio.WBP_Radio_C|GetIsSliderOn _radioui))
  (if (Variables|Default|GetCanUseUI)
    (Default|ToggleSlider _radioui)
    (if (and (!= _currprogress 0) (!= _currprogress 1))
      (bind _asbp_lighthouse_player_controller (Utilities|Casting|CastToBP_LighthousePlayerController (Pawn|GetController)))
      (Variables|/Script/Engine.PlayerController|SetbShowMouseCursor _asbp_lighthouse_player_controller _isslideron)
      (Variables|Default|SetShowMouse _isslideron))
    (if _isslideron
      (Audio|Components|Audio|Play _radiobackgroundnoise 0.0)
      (Default|DoOnceDialogue (Variables|Default|GetRadioUI))
      (else
        (Audio|Components|Audio|Stop _radiobackgroundnoise)))))

(event Custom|HandleWheelInput
  (params (WheelVal :type Float%20%28single-precision%29))
  (bind _radioui (Variables|Default|GetRadioUI))
  (if (Variables|Default|GetCanUseUI)
    (if (Variables|/Game/Ken_Playground/ClickableUI/WBP_Radio.WBP_Radio_C|GetIsSliderOn _radioui)
      (Default|ReceivefromWheel _radioui WheelVal))))

(event Custom|HandleRightMouseClick
  (bind _popupui (Variables|Default|GetPopUpUI))
  (if (Variables|Default|GetCanUseUI)
    (if (Variables|/Game/Ken_Playground/ClickableUI/WBP_KeyObjectWidget.WBP_KeyObjectWidget_C|GetIsUIOpen _popupui)
      _
      (else
        _))
    (Default|GoBacktoCam _popupui)))

(event Custom|LightsOn
  (Utilities|FlowControl|Sequence
    (:then_0
      (Rendering|Components|Light|SetIntensity (Variables|Default|GetPointLight1) 3e+03))
    (:then_1
      (Rendering|Components|Light|SetIntensity (Variables|Default|GetPointLight) 3e+03))
    (:then_2
      (Rendering|Components|Light|SetIntensity (Variables|Default|GetPointLight2) 3e+03))
    (:then_3
      (Rendering|Components|Light|SetIntensity (Variables|Default|GetPointLight3) 3e+03))
    (:then_4
      (Rendering|Components|Light|SetIntensity (Variables|Default|GetPointLight4) 3e+03))
    (:then_5
      (Rendering|Components|Light|SetIntensity (Variables|Default|GetSpotLight) 8e+03))))

(event Custom|PlayBGM
  (params (BGM :type Sound%20Wave%20Object%20Reference))
  (Audio|Components|Audio|SetSound (Variables|Default|GetBGM) BGM)
  (Audio|Components|Audio|Play (Variables|Default|GetBGM) 0.0))

(event Custom|StopRadioBackground
  (Audio|Components|Audio|Stop (Variables|Default|GetRadioBackgroundNoise)))

(event Custom|PlayRadioBackground
  (Audio|Components|Audio|Play (Variables|Default|GetRadioBackgroundNoise) 0.0))

(event Custom|StopBGM
  (Audio|Components|Audio|Stop (Variables|Default|GetBGM)))

(event EventBeginPlay
  (Audio|Components|Audio|Stop (Variables|Default|GetRadioBackgroundNoise))
  (bind _asbp_lighthouse_player_controller (Utilities|Casting|CastToBP_LighthousePlayerController (Pawn|GetController))
    (:then
      (Variables|/Script/Engine.PlayerController|SetbShowMouseCursor _asbp_lighthouse_player_controller true))
    (:CastFailed
      _))
  (Utilities|Array|Add (Variables|Default|GetIgnoreActors) self)
  (bind _returnvalue (UserInterface|CreateWidget "/Game/Ken_Playground/ClickableUI/WBP_FadeOutFadeIn.WBP_FadeOutFadeIn_C" (Game|GetPlayerController 0)))
  (bind _output_get (Variables|Default|SetFadeUI _returnvalue))
  (UserInterface|Viewport|AddtoViewport _output_get 6)
  (Widget|SetVisibility _output_get "Collapsed")
  (bind _returnvalue_2 (UserInterface|CreateWidget "/Game/Ken_Playground/ClickableUI/WBP_MainUI.WBP_MainUI_C"))
  (Variables|Default|SetPopUpUI (Variables|/Game/Ken_Playground/ClickableUI/WBP_MainUI.WBP_MainUI_C|GetWBP_KeyObjectWidget _returnvalue_2))
  (bind _output_get_2 (Variables|Default|SetRadioUI (Variables|/Game/Ken_Playground/ClickableUI/WBP_MainUI.WBP_MainUI_C|GetWBP_Radio _returnvalue_2)))
  (UserInterface|Viewport|AddtoViewport _returnvalue_2 4)
  (Widget|SetVisibility _returnvalue_2 "Visible")
  (bind _asbp_radio_subsystem (Utilities|Casting|CastToBP_RadioSubsystem (Subsystems|GetRadioSubsystem)))
  (Variables|/Game/Radio/BP_RadioSubsystem.BP_RadioSubsystem_C|SetRadioUI _asbp_radio_subsystem _output_get_2)
  (bind _asbp_lighthouse_player_controller_2 (Utilities|Casting|CastToBP_LighthousePlayerController (Pawn|GetController)))
  (EventDispatchers|BindEventtoOnMidMousClicked _asbp_lighthouse_player_controller_2 (EventDispatchers|CreateEvent :!event Custom|ToggleSlider))
  (EventDispatchers|BindEventtoOnMouseWheel _asbp_lighthouse_player_controller_2 (EventDispatchers|CreateEvent :!event Custom|HandleWheelInput))
  (EventDispatchers|BindEventtoOnRightMouseClicked _asbp_lighthouse_player_controller_2 (EventDispatchers|CreateEvent :!event Custom|HandleRightMouseClick)))

(event EventTick
  (params (DeltaSeconds :type Float%20%28single-precision%29))
  (bind _spotlight (Variables|Default|GetSpotLight))
  (bind _detectedpirate (Variables|Default|GetDetectedPirate))
  (bind _returnvalue (Transformation|GetWorldLocation _spotlight))
  (Utilities|FlowControl|Sequence
    (:then_0
      (bind _outhit (Collision|SphereTraceByChannel _returnvalue (+ _returnvalue (* (Math|Vector|GetForwardVector _spotlight) (Variables|/Script/Engine.LocalLightComponent|GetAttenuationRadius _spotlight))) 5e+01 "TraceTypeQuery1" false (Variables|Default|GetIgnoreActors) "ForOneFrame" false))
      (Utilities|Casting|CastToWaterBodyOcean (.HitActor (Collision|BreakHitResult _outhit))
        (:then
          (if (Utilities|IsValid _detectedpirate)
            (AI|Components|Blackboard|SetValueasBool (AI|GetBlackboard (AI|GetAIController _detectedpirate)) (Utilities|Name|MakeLiteralName "IsChasing") true))
          (bind _asbp_lighthouse_game_instance_subsystem (Utilities|Casting|CastToBP_LighthouseGameInstanceSubsystem (Subsystems|GetLightHouseGameInstanceSubsystem)))
          (for _array_element (Variables|/Game/Ken_Playground/Subsystems/BP_LighthouseGameInstanceSubsystem.BP_LighthouseGameInstanceSubsystem_C|GetControlledAIFollower _asbp_lighthouse_game_instance_subsystem)
            (if (Utilities|IsValid (AI|GetAIController _array_element))
              (AI|Components|Blackboard|SetValueasVector (AI|GetBlackboard (AI|GetAIController _array_element)) (Utilities|Name|MakeLiteralName "TargetLoc") (.ImpactPoint (Collision|BreakHitResult _outhit)))
              (bind _asbp_ship (Utilities|Casting|CastToBP_Ship _array_element))
              (bind _output_get (Variables|/Game/Ken_Playground/BP_Ship.BP_Ship_C|SetTargetLoc _asbp_ship (.ImpactPoint (Collision|BreakHitResult _outhit))))
              (Variables|Default|SetDebugShip _asbp_ship)
              (AI|SetFocalPoint (AI|GetAIController _array_element) _output_get)
              (AI|Components|Blackboard|SetValueasFloat (AI|GetBlackboard (AI|GetAIController _array_element)) (Utilities|Name|MakeLiteralName "DistToTarget") (Math|Vector|VectorLength (- (Transformation|GetActorLocation _asbp_ship) _output_get))))))
        (:CastFailed
          (bind _asbp_son_ship (Utilities|Casting|CastToBP_SonShip (.HitActor (Collision|BreakHitResult _outhit)))) ; Starts the capsize sequence when detected Son's Ship
        )))))

(event Input|KeyboardEvents|DebugKey2
  (params (Key :type Key%20Structure :default "None") (ActionValue :type Input%20Action%20Value%20Structure))
  (:Pressed
    (Class|RadioSubsystem|PlayFirstValidDollar (Subsystems|GetRadioSubsystem))))

(event Input|KeyboardEvents|DebugKey1
  (params (Key :type Key%20Structure :default "None") (ActionValue :type Input%20Action%20Value%20Structure))
  (:Pressed
    (Class|RadioSubsystem|PlayCurrentDollar (Subsystems|GetRadioSubsystem))))

(event Input|KeyboardEvents|DebugKeyE
  (params (Key :type Key%20Structure :default "None") (ActionValue :type Input%20Action%20Value%20Structure))
  (:Pressed
    (Default|DoSequentialCallouts (Variables|Default|GetRadioUI) "SonLastGoodWords")))

(event Input|MouseEvents|LeftMouseButton
  (params (Key :type Key%20Structure :default "None"))
  (bind _popupui (Variables|Default|GetPopUpUI))
  (bind _popupui_2 (Variables|Default|GetPopUpUI))
  (:Pressed
    (bind _asbp_lighthouse_player_controller (Utilities|Casting|CastToBP_LighthousePlayerController (Pawn|GetController)))
    (if (not (Variables|/Script/The_Lighthouse.LighthousePlayerController|GetbIsMainMenu _asbp_lighthouse_player_controller))
      (if (Variables|/Game/Ken_Playground/ClickableUI/WBP_KeyObjectWidget.WBP_KeyObjectWidget_C|GetIsUIOpen _popupui_2)
        (Default|HideAway _popupui_2)
        (else
          (bind _asbp_key_objects (Utilities|Casting|CastToBP_KeyObjects (.HitActor (Collision|BreakHitResult (.HitResult (Class|PlayerController|GetHitResultUnderCursorforObjects _asbp_lighthouse_player_controller (Utilities|Array|MakeArray "ObjectTypeQuery2" "ObjectTypeQuery4") true))))))
          (Default|SetImage _popupui_2)
          (bind _asbp_notebook_key_object (Utilities|Casting|CastToBP_NotebookKeyObject _asbp_key_objects)
            (:then
              (Default|UnlockRadio _asbp_notebook_key_object))
            (:CastFailed
              _))
          (Default|ReceivedInput _popupui (Variables|/Game/Ken_Playground/ClickableUI/BP_KeyObjects.BP_KeyObjects_C|GetText _asbp_key_objects) (Utilities|ResolveSoftReference (Variables|/Game/Ken_Playground/ClickableUI/BP_KeyObjects.BP_KeyObjects_C|GetStaticCamRef _asbp_key_objects)))
          (Default|SetImage _popupui (Variables|/Game/Ken_Playground/ClickableUI/BP_KeyObjects.BP_KeyObjects_C|GetTargetTexture _asbp_key_objects))
          (if (Variables|/Game/Ken_Playground/ClickableUI/BP_KeyObjects.BP_KeyObjects_C|GetIsCritical _asbp_key_objects)
            (if (not (Variables|/Game/Ken_Playground/ClickableUI/BP_KeyObjects.BP_KeyObjects_C|GetIsAccessed _asbp_key_objects))
              (Default|IncrementProgression _asbp_key_objects)
              (if (Variables|/Game/Ken_Playground/ClickableUI/BP_KeyObjects.BP_KeyObjects_C|GetIsRadio _asbp_key_objects)
                (Default|ShowRadioKey (Variables|Default|GetRadioUI))))))))))

(event Input|KeyboardEvents|3
  (params (Key :type Key%20Structure :default "None"))
  (:Pressed
    (Class|ProgressionSubsystem|ProgressGame (Subsystems|GetProgressionSubsystem))
    (bind _asbp_lighthouse_player_controller (Utilities|Casting|CastToBP_LighthousePlayerController (Pawn|GetController)))
    (Variables|/Script/The_Lighthouse.LighthousePlayerController|SetbIsLocked _asbp_lighthouse_player_controller false)))

(event Input|KeyboardEvents|R
  (params (Key :type Key%20Structure :default "None")))

(fn ConstructionScript)

(fn BPLighthousePawnAutoGenFunc)