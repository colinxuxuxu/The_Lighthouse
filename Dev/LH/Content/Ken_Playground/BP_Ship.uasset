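; Physics-driven ship that registers with the lighthouse game subsystem as a controlled AI follower and steers toward a target location.
; Tick yaws it by cross-product sign, using the negated right vector as forward, and flags when it faces the target.
; PhysicsMove pushes the mesh toward the target; UnpossessShip releases the AI controller, deregisters and heavily damps movement.
; The timeline-based RotateObject is deprecated.
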(event `self.ReceiveBeginPlay`
  (bind _asbp_lighthouse_game_instance_subsystem (cast `/Game/Ken_Playground/Subsystems/BP_LighthouseGameInstanceSubsystem` (subsystem `LightHouseGameInstanceSubsystem`)))
  (`/Game/Ken_Playground/Subsystems/BP_LighthouseGameInstanceSubsystem.AddToControlledAIFollower` _asbp_lighthouse_game_instance_subsystem self))

(event `SnapRotate`)

(event `self.ReceiveTick`
  (params (DeltaSeconds :type "Float (single-precision)"))
  (bind _staticmesh (`self.StaticMesh`))
  (bind _returnvalue (* DeltaSeconds (`self.RotateSpeed`)))
  (bind _shouldturnright (`self.FindCrossProduct`))
  (if _shouldturnright
    (`self.K2_AddActorLocalRotation` (`KismetMathLibrary.MakeRotator` 0.0 0.0 _returnvalue))
    (else
      (bind _result (`/Engine/EditorBlueprintResources/StandardMacros.NegateFloat` _returnvalue)
        (:`  `
          (`self.K2_AddActorLocalRotation` (`KismetMathLibrary.MakeRotator` 0.0 0.0 _result))))))
  (bind _angle (`self.CalculateAngleTick`))
  (if (<= _angle 10.0)
    (`PrimitiveComponent.SetAngularDamping` _staticmesh 1000.0)
    (`PrimitiveComponent.SetAngularDamping` _staticmesh 2.0)
    (set `self.IsFacingCorrectly` true)
    (else
      (`PrimitiveComponent.SetAngularDamping` _staticmesh 0.0)
      (set `self.IsFacingCorrectly` false))))

(event `PhysicsMove`
  (set `self.InitialLoc` (`self.K2_GetActorLocation`))
  (`PrimitiveComponent.AddForce` (`self.StaticMesh`) (* (`KismetMathLibrary.GetDirectionUnitVector` (`self.InitialLoc`) (`self.TargetLoc`)) (`self.Speed`)) "None" true))

(event `UnpossessShip`
  (bind _returnvalue (`AIBlueprintHelperLibrary.GetAIController` self))
  (if (`KismetSystemLibrary.IsValid` _returnvalue)
    (`Controller.UnPossess` _returnvalue))
  (bind _asbp_lighthouse_game_instance_subsystem (cast `/Game/Ken_Playground/Subsystems/BP_LighthouseGameInstanceSubsystem` (subsystem `LightHouseGameInstanceSubsystem`)))
  (`/Game/Ken_Playground/Subsystems/BP_LighthouseGameInstanceSubsystem.RemoveFromControlledAIFollower` _asbp_lighthouse_game_instance_subsystem self)
  (`PrimitiveComponent.SetLinearDamping` (`self.StaticMesh`) 100.0))

(event `SetLinearDamping`
  (params (Damping :type "Float (double-precision)" :default 1.0))
  (`PrimitiveComponent.SetLinearDamping` (`self.StaticMesh`) Damping))

(event `RotateObject`
  (bind _staticmesh (`self.StaticMesh`))
  ; Deprecated
  (bind _output_get (set `self.CachedLoc` (`self.TargetLoc`)))
  (bind _output_get_2 (set `self.InitialLoc` (`self.K2_GetActorLocation`)))
  (bind _out (`self.FindLookAt`))
  (`Timeline|T_Move` :!via `PlayFromStart`
    (:`Update`
      (bind _angle (`self.CalculateAngle`))
      (`KismetSystemLibrary.PrintString` (`KismetStringLibrary.Conv_DoubleToString` _angle))
      (if (<= _angle 15.0)
        (`PrimitiveComponent.SetAngularDamping` _staticmesh 1000.0)
        (`KismetSystemLibrary.Delay` 0.3)
        (`PrimitiveComponent.SetAngularDamping` _staticmesh 2.0)
        (else
          (`PrimitiveComponent.SetAngularDamping` _staticmesh 0.0)
          (`self.K2_SetActorRotation` (`KismetMathLibrary.RInterpTo` (`self.K2_GetActorRotation`) _out (`GameplayStatics.GetWorldDeltaSeconds`) 1.0)))))
    (:`Finished`
      (`self.TimelineFinished`))))

(fn `CalculateAngle`
  (returns (angle :type "Float (double-precision)"))
  (return (`KismetMathLibrary.DegAcos` (`KismetMathLibrary.Dot_VectorVector` (`KismetMathLibrary.NegateVector` (`self.GetActorRightVector`)) (`KismetMathLibrary.Normal` (- (`self.CachedLoc`) (`self.InitialLoc`)))))))

(fn `CalculateAngleTick`
  (returns (angle :type "Float (double-precision)"))
  (return (`KismetMathLibrary.DegAcos` (`KismetMathLibrary.Dot_VectorVector` (`KismetMathLibrary.NegateVector` (`self.GetActorRightVector`)) (`KismetMathLibrary.Normal` (- (`self.TargetLoc`) (`self.K2_GetActorLocation`)))))))

(fn `FindCrossProduct`
  (returns (ShouldTurnRight :type Boolean))
  (bind (_returnvalue_x _returnvalue_y _returnvalue_z) (`KismetMathLibrary.BreakVector` (`KismetMathLibrary.Cross_VectorVector` (`KismetMathLibrary.NegateVector` (`self.GetActorRightVector`)) (`KismetMathLibrary.Normal` (- (`self.TargetLoc`) (`self.K2_GetActorLocation`))))))
  (return (> _returnvalue_z 0.0)))

(fn `FindLookAt`
  (returns (Out :type "Rotator Structure"))
  (return (`KismetMathLibrary.FindLookAtRotation` (`self.GetActorRightVector`) (`KismetMathLibrary.Normal` (- (`self.CachedLoc`) (`self.InitialLoc`))))))

(fn `FindLookAtTick`
  (returns (Out :type "Rotator Structure"))
  (return (`KismetMathLibrary.FindLookAtRotation` (`self.GetActorRightVector`) (`KismetMathLibrary.Normal` (- (`self.TargetLoc`) (`self.K2_GetActorLocation`))))))

(fn `UserConstructionScript`
  (`StaticMeshComponent.SetStaticMesh` (`self.StaticMesh`) (`self.ObjMesh`)))