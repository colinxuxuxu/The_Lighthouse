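; One-shot trigger actor that stages the breakdown and capsizing of the son's ship.
; When BP_SonShip enters the box, it starts the "SonLastWords" radio callouts, locks the lighthouse pawn's UI and slider, unpossesses the ship, and raises its linear damping after a short delay.
; It listens to the radio subsystem's event and runs the stored ship's capsize sequence on "LastWord", timing the sinking to the dialogue.
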(event `self.ReceiveBeginPlay`
  (add `RadioSubsystem.OnEventRaised` (subsystem `RadioSubsystem`) (`|CreateDelegate` :!event `HandleOnEventRaised`)))

(event `self.Box.OnComponentBeginOverlap`
  (params (OverlappedComponent :type "PrimitiveComponent Object Reference") (OtherActor :type "Actor Object Reference") (OtherComp :type "PrimitiveComponent Object Reference") (OtherBodyIndex :type Integer) (bFromSweep :type Boolean) (SweepResult :type "HitResult Structure (by ref)"))
  (if (not (`self.IsUsed`))
    (bind _asbp_son_ship (cast `/Game/Ken_Playground/BP_SonShip` OtherActor))
    (set `self.ShipRef` _asbp_son_ship)
    (bind _asbp_lighthouse_pawn (cast `/Game/Lighthouse/BP_LighthousePawn` (`GameplayStatics.GetPlayerPawn` 0)))
    (bind _radioui (`/Game/Lighthouse/BP_LighthousePawn.RadioUI` _asbp_lighthouse_pawn))
    (`/Game/Ken_Playground/ClickableUI/WBP_Radio.DoSequentialCallouts` _radioui "SonLastWords")
    (set `/Game/Lighthouse/BP_LighthousePawn.CanUseUI` false _asbp_lighthouse_pawn)
    (`/Game/Ken_Playground/ClickableUI/WBP_Radio.ToggleSliderImages` _radioui "Collapsed")
    (`/Game/Ken_Playground/ClickableUI/WBP_Radio.SetSliderOff` _radioui)
    (`/Game/Ken_Playground/BP_Ship.UnpossessShip` _asbp_son_ship)
    (`KismetSystemLibrary.Delay` 1.0)
    (`/Game/Ken_Playground/BP_Ship.SetLinearDamping` _asbp_son_ship 1.0)
    (set `self.IsUsed` true)))

(event `HandleOnEventRaised`
  (params (EventName :type String))
  (if (`KismetStringLibrary.EqualEqual_StrStr` EventName "LastWord")
    (`/Game/Ken_Playground/BP_SonShip.CapsizeSequence` (`self.ShipRef`))))

(fn `UserConstructionScript`)