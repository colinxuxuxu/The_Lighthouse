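; Progression handler for the lighthouse game that stages the world as the story moves from evening through night, storm and son nights.
; It binds to the ProgressionSubsystem time delegate and switches on each new phase.
; Phases variously change music, smoothly shift BP_StylizedSky time or weather, unhide evening actors, toggle pawn lights and UI, activate the night camera, and spawn actors from class-to-transform maps.
; Directional light color and intensity tweaks remain but are disconnected.
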(event `self.ReceiveBeginPlay`
  (add `ProgressionSubsystem.TimeDelegate` (subsystem `ProgressionSubsystem`) (delegate `CustomEvent`))
  (bind _returnvalue (`GameplayStatics.GetActorOfClass` "/Script/Engine.DirectionalLight")) ; trying to find the directinoal light
  (set `self.DirLight` _returnvalue)
  (bind _returnvalue_2 (`GameplayStatics.GetActorOfClass` "/Game/SoStylized/Environment/Sky/BP_StylizedSky.BP_StylizedSky_C"))
  (bind _output_get (set `self.SkyVar` _returnvalue_2))
  (`/Game/SoStylized/Environment/Sky/BP_StylizedSky.Set Time ClockBased` _output_get 8.0 0.0 24.0 60.0)
  (bind _asbp_lighthouse_pawn (cast `/Game/Lighthouse/BP_LighthousePawn` (`GameplayStatics.GetPlayerPawn` 0)))
  (set `self.PlayerPawn` _asbp_lighthouse_pawn))

(event `CustomEvent`
  (params (CurrTime :type "DayProgression Enum" :default "Morning"))
  (bind _playerpawn (`self.PlayerPawn`))
  (switch `DayProgression` CurrTime
    (:`Evening`
      (`/Game/Lighthouse/BP_LighthousePawn.PlayBGM` _playerpawn "/Game/Sound/BGM/BGM_Morning.BGM_Morning") ; Evening BGM
      (for _array_element (`self.EveningUnhide`)
        (bind _output (`|ConvertAsset` _array_element))
        (if (`KismetSystemLibrary.IsValid` _output)
          (`/Game/Ken_Playground/ClickableUI/BP_KeyObjects.CheckProgression` _output)
          (`self.SetActorHiddenInGame` _output false)))
      (`/Game/SoStylized/Environment/Sky/BP_StylizedSky.SetTimeSmoothClockBased` (`self.SkyVar`) 17.0 0.0 24.0 60.0 0.7))
    (:`Night`
      (bind _asbp_lighthouse_player_controller (cast `/Game/Lighthouse/BP_LighthousePlayerController` (`GameplayStatics.GetPlayerController` 0)))
      (set `PlayerController.bShowMouseCursor` false _asbp_lighthouse_player_controller)
      (`/Game/Lighthouse/BP_LighthousePawn.PlayBGM` _playerpawn "/Game/Sound/BGM/BGM_Night1.BGM_Night1") ; Night BGM
      (`/Game/Lighthouse/BP_LighthousePawn.LightsOn` _playerpawn)
      (`self.SpawnObjects` (`self.NightObjectSpawnMap`))
      (bind _asbp_progression_subsystem (cast `/Game/Ken_Playground/Subsystems/BP_ProgressionSubsystem` (subsystem `ProgressionSubsystem`)))
      (`/Game/Ken_Playground/Subsystems/BP_ProgressionSubsystem.ActivateCam` _asbp_progression_subsystem "Night")
      (`/Game/SoStylized/Environment/Sky/BP_StylizedSky.SetTimeSmoothClockBased` (`self.SkyVar`) 22.0 0.0 24.0 60.0 0.7))
    (:`StormNight`
      (`self.SpawnObjects` (`self.StormNightObjectSpawn`)) ; Spawn the two ships
      (`/Game/Lighthouse/BP_LighthousePawn.PlayBGM` _playerpawn "/Game/Sound/BGM/BGM_Night1.BGM_Night1") ; Storm BGM
      (`/Game/SoStylized/Environment/Sky/BP_StylizedSky.Set Weather Smoothly` (`self.SkyVar`) "NewEnumerator3" 2.0))
    (:`StormNight2`
      (`self.SpawnObjects` (`self.StormNightSecondBoat`)))
    (:`SonNight`
      (`/Game/Lighthouse/BP_LighthousePawn.PlayBGM` _playerpawn "/Game/Sound/BGM/BGM_Night.BGM_Night") ; SonBGM
      (bind _asbp_lighthouse_pawn (cast `/Game/Lighthouse/BP_LighthousePawn` (`GameplayStatics.GetPlayerPawn` 0)))
      (`/Game/Lighthouse/BP_LighthousePawn.ToggleSliderUI` _asbp_lighthouse_pawn)
      (`self.SpawnObjects` (`self.SunShipSpawner`))
      (`/Game/SoStylized/Environment/Sky/BP_StylizedSky.Set Weather Smoothly` (`self.SkyVar`) "NewEnumerator2" 2.0))))

(event `SpawnObjects`
  (params (InputMap :type "Map of Actor Class Reference to Transform Structure"))
  (bind (_keypin _valuepin) (`|MapForEach` InputMap)
    (:`then`
      (`|SpawnActorFromClass` _keypin _valuepin "AlwaysSpawn" "MultiplyWithRoot" null null))))

(event `PlayFade`
  (bind _asbp_lighthouse_pawn (cast `/Game/Lighthouse/BP_LighthousePawn` (`GameplayStatics.GetPlayerPawn` 0)))
  (`/Game/Ken_Playground/ClickableUI/WBP_FadeOutFadeIn.PlayFade` (`/Game/Lighthouse/BP_LighthousePawn.FadeUI` _asbp_lighthouse_pawn)))

(fn `UserConstructionScript`)