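; Key object actor that feeds the game's progression count through ProgressionSubsystem.
; On BeginPlay, an instance that is not hidden and is marked IsCritical adds itself to TargetKeyCount.
; IncrementProgression raises CurrCount on every call for critical objects, while IsAccessed limits the subsystem's CheckProgress to the first call.
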(event `self.ReceiveBeginPlay`
  (if (not (`self.bHidden`))
    (`self.CheckProgression`)))

(event `IncrementProgression`
  (bind _returnvalue (subsystem `ProgressionSubsystem`))
  (if (`self.IsCritical`)
    (`/Engine/EditorBlueprintResources/StandardMacros.IncrementInt` (`ProgressionSubsystem.CurrCount` _returnvalue)
      (:`  `
        (if (not (`self.IsAccessed`))
          (`ProgressionSubsystem.CheckProgress` _returnvalue)
          (set `self.IsAccessed` true))))))

(event `CheckProgression`
  (if (`self.IsCritical`)
    (`/Engine/EditorBlueprintResources/StandardMacros.IncrementInt` (`ProgressionSubsystem.TargetKeyCount` (subsystem `ProgressionSubsystem`)))))

(fn `UserConstructionScript`)