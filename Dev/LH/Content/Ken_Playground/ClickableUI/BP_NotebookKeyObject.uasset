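; BP_NotebookKeyObject is a notebook key object that unlocks the radio.
; Its UnlockRadio event casts player controller 0 to BP_LighthousePlayerController and sets IsLocked to false.
; The event has no caller in this graph, and the construction script only runs the parent version.
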(event `UnlockRadio`
  (bind _asbp_lighthouse_player_controller (cast `/Game/Lighthouse/BP_LighthousePlayerController` (`GameplayStatics.GetPlayerController` 0)))
  (set `LighthousePlayerController.bIsLocked` false _asbp_lighthouse_player_controller))

(fn `UserConstructionScript`
  (`parent.UserConstructionScript`))