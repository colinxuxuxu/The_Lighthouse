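; BP_PirateShip is an AI-controlled pirate ship that chases a target and evades using physics forces on its static mesh.
; On BeginPlay it registers with the lighthouse subsystem's AI targeter and writes BP_Ship to the blackboard's TargetActor key.
; ChaseTarget accelerates toward a given actor, while Evade zeroes velocity and applies a random horizontal acceleration.
; A rotation update exists but is unconnected.
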(event `self.ReceiveBeginPlay`
  (bind _asbp_lighthouse_game_instance_subsystem (cast `/Game/Ken_Playground/Subsystems/BP_LighthouseGameInstanceSubsystem` (subsystem `LightHouseGameInstanceSubsystem`)))
  (`/Game/Ken_Playground/Subsystems/BP_LighthouseGameInstanceSubsystem.AddToControlledAITargeter` _asbp_lighthouse_game_instance_subsystem self)
  (set `self.Speed` 900.0)
  (bind _returnvalue (`GameplayStatics.GetActorOfClass` "/Game/Ken_Playground/BP_Ship.BP_Ship_C"))
  (`BlackboardComponent.SetValueAsObject` (`AIBlueprintHelperLibrary.GetBlackboard` (`AIBlueprintHelperLibrary.GetAIController` self)) "TargetActor" _returnvalue))

(event `ChaseTarget`
  (params (Target :type "Actor Object Reference"))
  (set `self.InitialLoc` (`self.K2_GetActorLocation`))
  (if (`KismetSystemLibrary.IsValid` Target)
    (bind _output_get (set `self.TargetLoc` (`self.K2_GetActorLocation` Target)))
    (`PrimitiveComponent.AddForce` (`self.StaticMesh`) (* (`KismetMathLibrary.GetDirectionUnitVector` (`self.InitialLoc`) _output_get) (`self.Speed`)) "None" true)))

(event `Evade`
  (bind _staticmesh (`self.StaticMesh`))
  (bind (_returnvalue_x _returnvalue_y) (`KismetMathLibrary.BreakVector` (* (`KismetMathLibrary.RandomUnitVector`) (`self.EvadeSpeed`))))
  (`PrimitiveComponent.SetPhysicsLinearVelocity` _staticmesh (0.0 0.0 0.0) false "None")
  (`PrimitiveComponent.AddForce` _staticmesh (`KismetMathLibrary.MakeVector` _returnvalue_x _returnvalue_y) "None" true))

(fn `UserConstructionScript`
  (`parent.UserConstructionScript`))