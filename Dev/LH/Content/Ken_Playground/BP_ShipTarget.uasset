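; BP_ShipTarget is a trigger box that registers ships reaching their target in the harbor.
; On first overlap by an untriggered BP_Ship, it sends critical "ShipInHarbor" radio callouts through the radio subsystem.
; It then increments and checks the progression count, marks the ship triggered and unpossesses it.
; A storm-night check has empty branches, leaving the second-ship spawn disconnected.
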(event `self.Box.OnComponentBeginOverlap`
  (params (OverlappedComponent :type "PrimitiveComponent Object Reference") (OtherActor :type "Actor Object Reference") (OtherComp :type "PrimitiveComponent Object Reference") (OtherBodyIndex :type Integer) (bFromSweep :type Boolean) (SweepResult :type "HitResult Structure (by ref)"))
  (bind _returnvalue (subsystem `ProgressionSubsystem`))
  (bind _returnvalue_2 (subsystem `RadioSubsystem`))
  (bind _asbp_ship (cast `/Game/Ken_Playground/BP_Ship` OtherActor)) ; if it's a ship we add to target progression
  (if (not (`/Game/Ken_Playground/BP_Ship.Triggered` _asbp_ship))
    (bind _returnvalue_3 (`RadioSubsystem.DoCallouts` _returnvalue_2 "ShipInHarbor" true))
    (bind _asbp_radio_subsystem (cast `/Game/Radio/BP_RadioSubsystem` _returnvalue_2))
    (`/Game/Radio/BP_RadioSubsystem.ReceiveCallouts` _asbp_radio_subsystem _returnvalue_3)
    (if (`|EnumEquality` (`ProgressionSubsystem.CurrProgress` _returnvalue) "StormNight")
      _
      (else
        _))
    (if (not (`/Game/Ken_Playground/BP_Ship.Triggered` _asbp_ship))
      (`/Engine/EditorBlueprintResources/StandardMacros.IncrementInt` (`ProgressionSubsystem.CurrCount` _returnvalue)
        (:`  `
          (`ProgressionSubsystem.CheckProgress` _returnvalue)
          (set `/Game/Ken_Playground/BP_Ship.Triggered` true _asbp_ship)
          (`/Game/Ken_Playground/BP_Ship.UnpossessShip` _asbp_ship))))))

(fn `UserConstructionScript`)