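; BP_SonShip is an AI follower ship in the lighthouse game that registers itself with the game instance subsystem on BeginPlay.
; Its CapsizeSequence event waits, then switches the player pawn's radio noise to a no-human sound and stops the music.
; It capsizes once by disabling buoyancy and applying physics impulses, then fades the player's screen.
; Logic to unpossess and unregister the ship is present but unconnected.
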(event `self.ReceiveBeginPlay`
  (bind _asbp_lighthouse_game_instance_subsystem (cast `/Game/Ken_Playground/Subsystems/BP_LighthouseGameInstanceSubsystem` (subsystem `LightHouseGameInstanceSubsystem`)))
  (`/Game/Ken_Playground/Subsystems/BP_LighthouseGameInstanceSubsystem.AddToControlledAIFollower` _asbp_lighthouse_game_instance_subsystem self))

(event `CapsizeSequence`
  (bind _staticmesh (`self.StaticMesh`))
  (`KismetSystemLibrary.Delay` 5.0)
  (bind _asbp_lighthouse_pawn (cast `/Game/Lighthouse/BP_LighthousePawn` (`GameplayStatics.GetPlayerPawn` 0)))
  (bind _radiobackgroundnoise (`/Game/Lighthouse/BP_LighthousePawn.RadioBackgroundNoise` _asbp_lighthouse_pawn))
  (`AudioComponent.SetSound` _radiobackgroundnoise "/Game/Sound/BGM/RadioBackgroundNoHuman.RadioBackgroundNoHuman")
  (`AudioComponent.Play` _radiobackgroundnoise 0.0)
  (`/Game/Lighthouse/BP_LighthousePawn.StopBGM` _asbp_lighthouse_pawn)
  (if (not (`self.IsCapsized`))
    (`ActorComponent.Deactivate` (`self.Buoyancy`))
    (`PrimitiveComponent.WakeRigidBody` _staticmesh "None")
    (`PrimitiveComponent.AddImpulse` _staticmesh (* (`self.GetActorUpVector`) 50000.0) "None" false)
    (`PrimitiveComponent.AddAngularImpulseInDegrees` (`self.StaticMesh`) (* (`self.GetActorRightVector`) 1000000.0) "None" false)
    (set `self.IsCapsized` true)
    (`ActorComponent.K2_DestroyComponent` (`self.Buoyancy`))
    (`KismetSystemLibrary.Delay` 6.0)
    (`/Game/Ken_Playground/ClickableUI/WBP_FadeOutFadeIn.PlayFade` (`/Game/Lighthouse/BP_LighthousePawn.FadeUI` _asbp_lighthouse_pawn))))

(fn `UserConstructionScript`
  (`parent.UserConstructionScript`))